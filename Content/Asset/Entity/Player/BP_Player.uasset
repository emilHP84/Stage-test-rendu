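; BP_Player is the player Blueprint, tracking the player's life and death state.
; BeginPlay fills current life from max life and clears the dead flag, and TakeDamage subtracts damage without clamping.
; Tick polls current life and calls OnDeath on every frame it is at or below zero.
; OnDeath only sets IsDead, with no further death handling.
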(event `self.ReceiveBeginPlay`
  ; set la current life
  (set `self.Player_CurrentLife` (`self.Player_maxLife`))
  (set `self.IsDead` false))

(event `self.ReceiveTick`
  (params (DeltaSeconds :type "Float (single-precision)"))
  ; verifie si la vie <= 0
  (if (<= (`self.Player_CurrentLife`) 0)
    (`self.OnDeath`)))

(fn `OnDeath`
  (set `self.IsDead` true))

(fn `TakeDamage`
  (params (damage :type Integer))
  (set `self.Player_CurrentLife` (- (`self.Player_CurrentLife`) damage)))

(fn `UserConstructionScript`)