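; Entity character Blueprint that follows the player and can deal damage to it.
; Each Tick calls FollowPlayer, which snaps the entity to the player's location and applies a look-at rotation while CanFollow is set.
; DetectPlayerDistance toggles CanFollow by a small distance threshold, but it and FollowPlayer call each other with no exit while the player cast succeeds.
; AttackPlayer applies EntityDamage to the player but is not called in this Blueprint.
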(event `self.ReceiveTick`
  (params (DeltaSeconds :type "Float (single-precision)"))
  (`self.FollowPlayer`)
  (`self.DetectPlayerDistance` 2.0))

(fn `AttackPlayer`
  (`/Game/Asset/Entity/Player/BP_Player.TakeDamage` (`self.PlayerRef`) (`self.Entity_Damage`)))

(fn `DetectPlayerDistance`
  (params (DetectDistance :type "Float (double-precision)" :default 2.0))
  ; récupération de la location (player)
  (bind _asbp_player (cast `/Game/Asset/Entity/Player/BP_Player` (`self.PlayerRef`)))
  ; check si la distance est > à minimalDistance
  (if (< (`KismetMathLibrary.Vector_Distance` (`KismetMathLibrary.TransformLocation` (`self.GetTransform` self)) (`KismetMathLibrary.TransformLocation` (`self.GetTransform` _asbp_player))) DetectDistance)
    ; application
    (`self.FollowPlayer`)
    (set `self.CanFollow` false)
    (else
      (`self.FollowPlayer`)
      (set `self.CanFollow` true))))

(fn `FollowPlayer`
  (bind _returnvalue (`self.K2_GetActorLocation` (`self.PlayerRef`)))
  ; verification des autorisation
  (if (and (`KismetSystemLibrary.IsValid` (`self.PlayerRef`)) (`self.CanFollow`))
    ; application de la rotation & de la location
    (`self.K2_SetActorLocation` _returnvalue)
    (`self.K2_SetActorRotation` (`KismetMathLibrary.FindLookAtRotation` (`self.K2_GetActorLocation`) _returnvalue)))
  (`self.DetectPlayerDistance` 2.0))

(fn `UserConstructionScript`)